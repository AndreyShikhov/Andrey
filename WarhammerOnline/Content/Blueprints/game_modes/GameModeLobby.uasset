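; Lobby game mode that tracks connected players, server settings and chat history for a multiplayer lobby.
; On login it copies server settings from the Create_lobby game instance to the joining LobbyPlayerController and replays logged chat; joins and leaves are announced as server messages.
; Each roster change rebuilds every client's player list with Steam avatars and counts.
; It also kicks players by index and launches the selected map via console command.
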(event Custom|Add_Mesage_To_Chat_History
  (params (Data :type Chat%20Mesage%20Structure%20Structure))
  ;[1 1 1] Load Mesage-History
  (Utilities|Array|Add (Variables|Default|GetMesage_LOG) Data))

(event Custom|Send_Server_Mesage
  (params (Message :type String))
  ;[1 1 1] Push mesage to server
  (bind _aslobby_player_controller (Utilities|Casting|CastToLobbyPlayerController (Game|GetPlayerController 0)))
  (Default|AddMesagefromServertoEachePlayer _aslobby_player_controller Message (Utilities|Struct|MakeSlateColor "(R=1.000000,G=0.000000,B=1.000000,A=1.000000)") true))

(event Custom|Join_Game
  ;[1 1 1] join game
  (bind _array_element (Utilities|Array|ForEachLoopwithBreak (Variables|Default|GetAll_Maps) :!label _label)
    (:LoopBody
      (if (Utilities|Enum|Equal(Enum) _array_element (Variables|Default|GetServer_Map))
        (Utilities|FlowControl|Sequence
          (:then_0
            (goto _label Break))
          (:then_1
            (bind _output_get (Variables|Default|Setcomplite_path__to_map (Utilities|String|Append (Variables|Default|Getcomplite_path__to_map) (Variables|Default|GetServer_Map))))
            (Development|ExecuteConsoleCommand _output_get (Game|GetPlayerController 0))
            (bind _ascreate_lobby (Utilities|Casting|CastToCreate_lobby (Game|GetGameInstance)))
            (Default|JoinGame _ascreate_lobby)))))))

(event Custom|Update_Server
  ;[1 1 1] update Server
  (for _array_element (Variables|Default|GetAll_PCs)
    (bind _aslobby_player_controller (Utilities|Casting|CastToLobbyPlayerController _array_element))
    (Default|ClearPlayerList _aslobby_player_controller)
    (for (_array_element_2 _array_index) (Variables|Default|GetAll_PCs)
      (bind _returnvalue (Class|AdvancedSteamFriendsLibrary|GetSteamFriendAvatar (Class|AdvancedSessionsLibrary|GetUniqueNetID _array_element_2) "SteamAvatar_Small")
        (:OnSuccess
          (Variables|Default|SetFail false))
        (:AsyncLoading
          (Variables|Default|SetFail false))
        (:OnFailure
          (Variables|Default|SetFail true)))
      (Default|AddPlayer _aslobby_player_controller (Variables|Default|GetFail) (Utilities|Text|ToText(String) (Class|AdvancedSessionsLibrary|GetPlayerName _array_element_2)) _returnvalue _array_index)))
  (for _array_element_3 (Variables|Default|GetAll_PCs)
    (bind _aslobby_player_controller_2 (Utilities|Casting|CastToLobbyPlayerController _array_element_3))
    (Default|UpdateNumbersOfPlayers _aslobby_player_controller_2 (Utilities|Array|Length (Variables|Default|GetAll_PCs)))))

(event Custom|Kick_Player
  (params (Index :type Integer))
  ;[1 1 1] Kick player
  (bind _aslobby_player_controller (Utilities|Casting|CastToLobbyPlayerController (Utilities|Array|Get(acopy) (Variables|Default|GetAll_PCs) Index)))
  (Default|KickPlayer _aslobby_player_controller))

(event EventOnLogout
  (params (ExitingController :type Controller%20Object%20Reference))
  (bind _all_pcs (Variables|Default|GetAll_PCs))
  ;[1 1 1] logout
  (bind (_array_element _array_index) (Utilities|Array|ForEachLoopwithBreak _all_pcs :!label _label)
    (:LoopBody
      (if (== ExitingController _array_element)
        (CallFunction|SendServerMesage (Utilities|String|Append (Class|AdvancedSessionsLibrary|GetPlayerName _array_element) " : Left"))
        (goto _label Break)))
    (:Completed
      (Utilities|Array|RemoveIndex _all_pcs _array_index)
      (CallFunction|UpdateServer))))

(event EventPostLogin
  (params (NewPlayer :type Player%20Controller%20Object%20Reference))
  ;[1 1 1] Set lobby param
  (CallFunction|SendServerMesage (Utilities|String|Append (Class|AdvancedSessionsLibrary|GetPlayerName NewPlayer) " : Joined"))
  (Networking|SwitchHasAuthority
    (:Authority
      (Utilities|Array|Add (Variables|Default|GetAll_PCs) NewPlayer)
      (bind _ascreate_lobby (Utilities|Casting|CastToCreate_lobby (Game|GetGameInstance)))
      (Variables|Default|SetServer_Name (Variables|/Game/Blueprints/instance/Create_lobby.Create_lobby_C|GetServer_Name _ascreate_lobby))
      (Variables|Default|SetServer_Map (Variables|/Game/Blueprints/instance/Create_lobby.Create_lobby_C|GetServer_Map _ascreate_lobby))
      (Variables|Default|SetServer_Mode (Variables|/Game/Blueprints/instance/Create_lobby.Create_lobby_C|GetServer_Mode _ascreate_lobby))
      (Variables|Default|SetServer_Slots (Variables|/Game/Blueprints/instance/Create_lobby.Create_lobby_C|GetServer_Slots _ascreate_lobby))
      ;[1 1 1] add lobby and set to lobby param
      (bind _aslobby_player_controller (Utilities|Casting|CastToLobbyPlayerController NewPlayer))
      (Default|AddLobby _aslobby_player_controller (Variables|Default|GetServer_Name) (Variables|Default|GetServer_Map) (Variables|Default|GetServer_Mode) (Variables|Default|GetServer_Slots))
      (CallFunction|UpdateServer)
      ;[1 1 1] Load Mesage-History
      (for _array_element (Variables|Default|GetMesage_LOG)
        (bind _aslobby_player_controller_2 (Utilities|Casting|CastToLobbyPlayerController NewPlayer))
        (Default|AddMesagetoChat _aslobby_player_controller_2 _array_element)))))

(fn ConstructionScript)