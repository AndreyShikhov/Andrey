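; LobbyPlayerController is the player controller for a multiplayer lobby, acting as the bridge to that player's lobby UI.
; Add_Lobby shows the cursor and creates the Lobby_menu widget with the server's name, map, mode and slots.
; Other events forward player list and count updates to that widget, or swap it for a loading screen.
; Kick_Player opens the Menu level and destroys the session.
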(event Custom|Add_Lobby
  (params (Server_Name :type String) (Server_Map :type String) (Server_Mode :type String) (Server_Slots :type Integer))
  ;[1 1 1] Create menu lobby widget
  (Variables|Default|SetbShowMouseCursor true)
  (bind _returnvalue (UserInterface|CreateWidget "/Game/UI/Lobby/Lobby_menu.Lobby_menu_C" 0 (Utilities|Text|ToText(String) Server_Name) (Utilities|Text|ToText(String) Server_Map) (Utilities|Text|ToText(String) Server_Mode) Server_Slots))
  (bind _output_get (Variables|Default|SetLobby _returnvalue))
  (UserInterface|Viewport|AddtoViewport _output_get 1))

(event Custom|Loading_Screen
  ;[1 1 1] show loaing screen
  (Widget|RemovefromParent (Variables|Default|GetLobby))
  (bind _returnvalue (UserInterface|CreateWidget "/Game/UI/Lobby/Loading_screen.Loading_screen_C" self))
  (UserInterface|Viewport|AddtoViewport _returnvalue 0))

(event Custom|Add_Player
  (params (isFail :type Boolean) (Player :type Text) (Avatar :type Texture%202D%20Object%20Reference) (PlayerIndex :type Integer))
  (Default|AddPlayertoList (Variables|Default|GetLobby) isFail Player Avatar PlayerIndex))

(event Custom|Clear_Player_List
  (Default|ClearPlayerList (Variables|Default|GetLobby)))

(event Custom|Kick_Player
  (Game|OpenLevel(byName) "Menu")
  (|DestroySession self))

(event Custom|Update_Numbers_Of_Players
  (params (current_Players :type Integer))
  (Variables|/Game/UI/Lobby/Lobby_menu.Lobby_menu_C|Setcurrent_Players (Variables|Default|GetLobby) current_Players))

(fn ConstructionScript)