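; Lobby Blueprint that hosts multiplayer sessions and persists the player's LAN name.
; Createlobby stores the server settings and creates an Advanced Session with name, map, mode, LAN and password properties, then opens the default level as a listen server.
; JoinGame currently only destroys the existing session, without joining another.
; Save and load events keep the LAN name in a SaveGame slot, with a function to check it exists.
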(event Custom|Create%20lobby
  (params (Server_Name :type String) (Server_Map :type String) (Server_Slots :type Integer) (Server_Mode :type String) (Server_Method_is_Lan? :type Boolean) (Is_Password :type Boolean) (Password :type String))
  ;[1 1 1] Set param for lobby
  (Variables|Parametrtolobby|SetServer_Name Server_Name)
  (Variables|Parametrtolobby|SetServer_Map Server_Map)
  (Variables|Parametrtolobby|SetServer_Slots Server_Slots)
  (Variables|Parametrtolobby|SetServer_Mode Server_Mode)
  (Variables|Parametrtolobby|SetServer_Method_is_Lan? Server_Method_is_Lan?)
  (Variables|Parametrtolobby|SetIs_Password Is_Password)
  (Variables|Parametrtolobby|SetPassword Password)
  ;[1 1 1] Create lobby
  (|AdvancedSession (Utilities|Array|MakeArray (Class|AdvancedSessionsLibrary|MakeLiteralSessionPropertyString "NAME" (Variables|Parametrtolobby|GetServer_Name)) (Class|AdvancedSessionsLibrary|MakeLiteralSessionPropertyString "MAP" (Variables|Parametrtolobby|GetServer_Map)) (Class|AdvancedSessionsLibrary|MakeLiteralSessionPropertyString "MODE" (Variables|Parametrtolobby|GetServer_Mode)) (Class|AdvancedSessionsLibrary|MakeLiteralSessionPropertyBool "LAN" (Variables|Parametrtolobby|GetServer_Method_is_Lan?)) (Class|AdvancedSessionsLibrary|MakeLiteralSessionPropertyBool "ISPASSWORD" (Variables|Parametrtolobby|GetIs_Password)) (Class|AdvancedSessionsLibrary|MakeLiteralSessionPropertyString "PASSWORD" (Variables|Parametrtolobby|GetPassword))) (Game|GetPlayerController 0) (Variables|Parametrtolobby|GetServer_Slots) 0 (Variables|Parametrtolobby|GetServer_Method_is_Lan?) true false true true false false false true
    (:OnSuccess
      (Game|OpenLevel(byName) (Variables|Parametrtolobby|GetDefaul_Level) true "listen"))))

(event Custom|JoinGame
  ;[1 1 1] join game
  (|DestroySession (Game|GetPlayerController 0)))

(event Custom|Save_Player_Data
  (params (LAN_Name :type String))
  ;[1 1 1] save player data
  (bind _output_get (Variables|Default|SetLAN_Name LAN_Name))
  (bind _returnvalue (SaveGame|CreateSaveGameObject "/Game/Blueprints/Saves/Save_Player_Data.Save_Player_Data_C"))
  (Variables|/Game/Blueprints/Saves/Save_Player_Data.Save_Player_Data_C|SetLAN_Name _returnvalue _output_get)
  (SaveGame|SaveGametoSlot _returnvalue (Variables|Default|GetPlayer_Slot_SG)))

(event Custom|Load_Player_Data
  ;[1 1 1] load player data
  (bind _returnvalue (SaveGame|LoadGamefromSlot (Variables|Default|GetPlayer_Slot_SG)))
  (bind _assave_player_data (Utilities|Casting|CastToSave_Player_Data _returnvalue))
  (Variables|Default|SetLAN_Name (Variables|/Game/Blueprints/Saves/Save_Player_Data.Save_Player_Data_C|GetLAN_Name _assave_player_data)))

(fn IsPlayerDataExists
  (bind _returnvalue (SaveGame|DoesSaveGameExist (Variables|Default|GetPlayer_Slot_SG)))
  (return _returnvalue))